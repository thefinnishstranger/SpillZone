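; BP_Gameplay_PC is the gameplay player controller that owns and displays the local player's HUD.
; On BeginPlay, only for a local controller, it creates WB_Gameplay_HUD, stores it as WBHUD and adds it to the viewport.
; On UnPossess, if that HUD is valid, it removes just the health bar child widget from its parent, leaving the rest of the HUD in place.
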(event EventBeginPlay
  (|CallParentFunction)
  (if (Pawn|IsLocalPlayerController)
    (bind _returnvalue (UserInterface|CreateWidget "/Game/Widgets/GameWidgets/WB_Gameplay_HUD.WB_Gameplay_HUD_C" self))
    (bind _output_get (Variables|Default|SetWB_HUD _returnvalue))
    (UserInterface|Viewport|AddtoViewport _output_get 0)))

(event EventUnPossess
  (params (UnpossessedPawn :type Pawn%20Object%20Reference))
  (bind _wb_hud (Variables|Default|GetWB_HUD)
    (:then
      (Widget|RemovefromParent (Variables|/Game/Widgets/GameWidgets/WB_Gameplay_HUD.WB_Gameplay_HUD_C|GetWB_HealthBar _wb_hud)))
    (:else)))

(fn ConstructionScript
  (|CallParentFunction))