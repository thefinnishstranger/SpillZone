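; Battle royale game state that runs the match from pre-game countdown through shrinking zones to a declared winner.
; Enough connected players start the countdown, which at zero spawns the zone and airplanes, then a repeating timer shrinks the zone.
; Both countdowns self-loop through RepNotifies, with authority triggering each delayed decrement.
; Connections and deaths trigger a last-survivor check, while replicated kill feed and winner name drive UI.
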(event Custom|Match_CountDown
  (Utilities|FlowControl|Delay 1.0)
  (Variables|Default|SetMatchStart_Countdown (- (Variables|Default|GetMatchStart_Countdown) 1)))

(event Custom|CheckIfGameFinished?
  ;[1 1 1] Check if the game is finished
  (Networking|SwitchHasAuthority
    (:Authority
      (Utilities|FlowControl|Delay 1.0)
      (CallFunction|DetermineWinner))))

(event Custom|Countdown_Zone
  (Utilities|FlowControl|Delay 1.0)
  (Variables|Default|SetZone_Countdown (- (Variables|Default|GetZone_Countdown) 1)))

(event EventNotifyPlayerDeath
  (params (Killer :type String) (PlayerWhoDied :type String))
  ;[1 1 1] Decrease the amount of Survivors
  (Variables|Default|SetCurrentAmountOfPlayers (- (Variables|Default|GetCurrentAmountOfPlayers) 1))
  (Variables|Default|SetKillFeed (Utilities|String|Append Killer " killed " PlayerWhoDied))
  (CallFunction|CheckifGameFinished?))

(event EventNotifyPlayerConnection
  (bind _returnvalue (Class|GameplayStatics|GetNumPlayerStates))
  (Variables|Default|SetCurrentAmountOfPlayers _returnvalue)
  (CallFunction|CheckifGameFinished?)
  (if (>= _returnvalue (Variables|Default|GetMinimumRequiredPlayers))
    (Utilities|FlowControl|DoOnce false
      (:Completed
        (Variables|Default|SetMatchStart_Countdown (Variables|Default|GetDefault_MatchCountdown))))))

(fn ConstructionScript
  (|CallParentFunction))

(fn OnRepMatchStartCountdown
  (CallFunction|UpdateMatchStartCountdownWidget)
  (Networking|SwitchHasAuthority
    (:Authority
      (if (== (Variables|Default|GetMatchStart_Countdown) 15)
        (CallFunction|MatchCountDown)
        (elif (== (Variables|Default|GetMatchStart_Countdown) 0)
          (bind _outactors (Actor|GetAllActorsOfClass "/Game/Blueprints/Actors/Zone/BP_ZoneSpawner.BP_ZoneSpawner_C"))
          (Default|SpawnZone (Utilities|Array|Get(acopy) _outactors))
          (Variables|Default|SetZone_Countdown (Variables|Default|GetTimeBetweenZones))
          (bind _outactors_2 (Actor|GetAllActorsOfClass "/Game/Blueprints/Actors/BP_AirplaneSpawner.BP_AirplaneSpawner_C"))
          (for _array_element _outactors_2
            (Default|SpawnAirplane _array_element))
          (else
            (CallFunction|MatchCountDown)))))))

(fn UpdateMatchStartCountdownWidget
  (bind _foundwidgets (Widget|GetAllWidgetsOfClass "/Game/Widgets/GameWidgets/WB_MatchStartCountdown.WB_MatchStartCountdown_C" false))
  (for _array_element _foundwidgets
    (Default|UpdateWidget _array_element (Variables|Default|GetMatchStart_Countdown))))

(fn OnRepKillFeed
  (CallFunction|AddKillFeed (Utilities|Text|ToText(String) (Variables|Default|GetKillFeed))))

(fn OnRepWinnerName
  (if (not (Utilities|Array|IsEmpty (Variables|Default|GetWinnerName)))
    (if (Pawn|IsLocalPlayerController (Game|GetPlayerController 0))
      (bind _returnvalue (UserInterface|CreateWidget "/Game/Widgets/GameWidgets/MatchResult/WB_MatchResult.WB_MatchResult_C" (Game|GetPlayerController 0) (Variables|Default|GetWinnerName)))
      (UserInterface|Viewport|AddtoViewport _returnvalue 0)
      (Variables|/Script/Engine.PlayerController|SetbShowMouseCursor (Game|GetPlayerController 0) true)
      (Input|SetInputModeGameandUI (Game|GetPlayerController 0) _returnvalue "DoNotLock" true))))

(fn DetermineWinner
  (if (== (Variables|Default|GetMatchStart_Countdown) 0)
    (bind _outactors (Actor|GetAllActorsOfClass "/Game/Blueprints/GameModes/Gameplay/BP_Gameplay_Character.BP_Gameplay_Character_C"))
    (if (== (Utilities|Array|Length _outactors) 1)
      (Variables|Default|SetWinnerName (PlayerState|GetPlayerName (Variables|/Script/Engine.Pawn|GetPlayerState (Utilities|Array|Get(acopy) _outactors)))))))

(fn OnRepZoneCountdown
  (Networking|SwitchHasAuthority
    (:Authority
      (if (Utilities|Array|IsEmpty (Variables|Default|GetWinnerName))
        (if (== (Variables|Default|GetZone_Countdown) 0)
          (Variables|Default|SetZone_Countdown (Variables|Default|GetTimeBetweenZones))
          (bind _outactors (Actor|GetAllActorsOfClass "/Game/Blueprints/Actors/Zone/BP_Zone.BP_Zone_C"))
          (Default|Shrink (Utilities|Array|Get(acopy) _outactors))
          (else
            (CallFunction|CountdownZone)))))))