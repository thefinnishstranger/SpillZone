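; BP_Zone is a shrinking play-area actor that tracks whether gameplay characters are inside or outside it.
; Each Shrink call sets a target size a fixed step below the zone mesh's current scale, clamped at zero.
; Tick slowly interpolates the mesh's uniform scale toward that target.
; Begin and end overlaps feed HandleZoneLogic, which sets OutsideZone on BP_Gameplay_Character with authority only.
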(event OnComponentBeginOverlap(SM_Zone)
  (params (OverlappedComponent :type Primitive%20Component%20Object%20Reference) (OtherActor :type Actor%20Object%20Reference) (OtherComp :type Primitive%20Component%20Object%20Reference) (OtherBodyIndex :type Integer) (bFromSweep :type Boolean) (SweepResult :type Hit%20Result%20Structure%20%28by%20ref%29))
  (CallFunction|HandleZoneLogic OtherActor false))

(event OnComponentEndOverlap(SM_Zone)
  (params (OverlappedComponent :type Primitive%20Component%20Object%20Reference) (OtherActor :type Actor%20Object%20Reference) (OtherComp :type Primitive%20Component%20Object%20Reference) (OtherBodyIndex :type Integer))
  (CallFunction|HandleZoneLogic OtherActor true))

(event Custom|Shrink
  (Variables|Default|SetTargetSize (Math|Float|Clamp(Float) (- (.x (Transformation|GetWorldScale (Variables|Default|GetSM_Zone))) 2.5e+02) 0.0 1e+03)))

(event EventBeginPlay
  (Networking|SwitchHasAuthority
    (:Authority
      (Variables|Default|SetTargetSize (.x (Transformation|GetWorldScale (Variables|Default|GetSM_Zone)))))))

(event EventTick
  (params (DeltaSeconds :type Float%20%28single-precision%29))
  (bind _targetsize (Variables|Default|GetTargetSize))
  (bind _sm_zone (Variables|Default|GetSM_Zone))
  (bind _returnvalue (Transformation|GetWorldScale _sm_zone))
  (bind _returnvalue_2 (Math|Interpolation|FInterpTo (.x _returnvalue) _targetsize DeltaSeconds 0.1))
  (if (not (== (.x _returnvalue) 0.0))
    (Transformation|SetWorldScale3D (Variables|Default|GetSM_Zone) (Math|Vector|MakeVector _returnvalue_2 _returnvalue_2 _returnvalue_2))))

(fn ConstructionScript)

(fn HandleZoneLogic
  (params (OtherActor :type Object%20Object%20Reference) (OutsideZone? :type Boolean))
  (Networking|SwitchHasAuthority
    (:Authority
      (if (== (Utilities|GetClass OtherActor) "/Game/Blueprints/GameModes/Gameplay/BP_Gameplay_Character.BP_Gameplay_Character_C")
        (bind _asbp_gameplay_character (Utilities|Casting|CastToBP_Gameplay_Character OtherActor))
        (Variables|/Game/Blueprints/GameModes/Core/BP_Core_Character.BP_Core_Character_C|SetOutsideZone? _asbp_gameplay_character OutsideZone?)))))