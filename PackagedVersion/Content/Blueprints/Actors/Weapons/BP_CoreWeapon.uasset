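; Base weapon actor for a character, providing networked automatic hitscan fire, ammo and timed reload.
; Input calls server events that loop a fire timer, with a negative start delay for an immediate first shot, or refill ammo after a delay.
; Shots trace from the owner's camera, offset forward by spring arm length, and apply damage.
; Multicasts play sounds, timeline-driven recoil and reload motion, and Niagara impacts.
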(event Custom|Shoot
  ;[1 1 1] Shooting
  (Utilities|CanShoot?
    (:true
      (Math|Integer|DecrementInt (Variables|Default|GetAmmo)
        (:%20%20
          (CallFunction|MCShoot)
          (CallFunction|LineTraceShot))))))

(event Custom|MC_SpawnImpact
  (params (Location :type Vector) (Normal :type Vector))
  ;[1 1 1] Shooting
  (Niagara|SpawnSystematLocation "/Game/Assets/Niagara/NS_Impact.NS_Impact" Location (Math|Conversions|RotationFromXVector Normal)))

(event Custom|SR_Reload
  ;[1 1 1] Reload
  (Utilities|CanReload?
    (:true
      (Variables|Default|SetReloading? true)
      (CallFunction|MCReload)
      (Utilities|FlowControl|Delay (Variables|Default|GetReloadDuration))
      (Variables|Default|SetAmmo (Variables|Default|GetMaxAmmo))
      (Variables|Default|SetReloading? false))))

(event Custom|MC_Reload
  ;[1 1 1] Reload
  (Audio|SpawnSoundAttached (Variables|Default|GetReloadSoundEffect) (Variables|Default|GetStaticMesh) "None" "0, 0, 0" "0, 0, 0" "KeepRelativeOffset" false 1.0 1.0 0.0 0 0)
  (Components|Timeline|SetPlayRate (Variables|Default|GetTL_Reload) (Variables|Default|GetReloadDuration))
  (bind _rotation (Timeline|TL_Reload PlayFromStart)
    (:Update
      (Transformation|SetRelativeRotation (Variables|Default|GetStaticMesh) (Math|Rotator|MakeRotator _rotation 0.0 0.0) false false))))

(event Custom|SR_PrimaryAction
  (params (Pressed? :type Boolean))
  (bind _rateoffire (Variables|Default|GetRateOfFire))
  ;[1 1 1] Shooting
  (if Pressed?
    (bind _returnvalue (Utilities|Time|SetTimerbyEvent (delegate Custom|Shoot) _rateoffire true (* _rateoffire -1.0)))
    (Variables|Default|SetTH_Shooting _returnvalue)
    (else
      (Utilities|Time|ClearandInvalidateTimerbyHandle (Variables|Default|GetTH_Shooting)))))

(event Custom|MC_Shoot
  ;[1 1 1] Shooting
  (Audio|SpawnSoundAttached (Variables|Default|GetShootingSoundEffect) (Variables|Default|GetStaticMesh) "None" "0, 0, 0" "0, 0, 0" "KeepRelativeOffset" false 1.0 1.0 0.0 0 0)
  (bind (_direction _recoil _location) (Timeline|TL_AnimateWeapon PlayFromStart)
    (:Update
      (Transformation|SetRelativeRotation (Variables|Default|GetStaticMesh) (Math|Rotator|MakeRotator _recoil 0.0 0.0) false false)
      (Transformation|SetRelativeLocation (Variables|Default|GetStaticMesh) (Math|Vector|MakeVector 0.0 _location 0.0) false false))))

(event EventInputPrimaryActionPressed
  ;[1 1 1] Inputs
  (CallFunction|SRPrimaryAction true))

(event EventInputPrimaryActionReleased
  ;[1 1 1] Inputs
  (CallFunction|SRPrimaryAction false))

(event EventInputReload
  ;[1 1 1] Reload
  (CallFunction|SRReload))

(event EventSetupActor
  (params (Character :type BP%20Core%20Character%20Object%20Reference))
  (Variables|Default|SetAs%20BP%20Core%20Character Character))

(fn ConstructionScript
  (Components|StaticMesh|SetStaticMesh (Variables|Default|GetStaticMesh) (Variables|Default|GetWeapon_Mesh)))

(fn LineTraceShot
  (bind _as_bp_core_character (Variables|Default|GetAs%20BP%20Core%20Character))
  (bind _camera (Variables|/Game/Blueprints/GameModes/Core/BP_Core_Character.BP_Core_Character_C|GetCamera _as_bp_core_character))
  (bind _returnvalue (Transformation|GetWorldLocation _camera))
  (bind _returnvalue_2 (Math|Vector|GetForwardVector _camera))
  (bind (_outhit _returnvalue_3) (Collision|LineTraceByChannel (+ _returnvalue (* _returnvalue_2 (Variables|/Script/Engine.SpringArmComponent|GetTargetArmLength (Variables|/Game/Blueprints/GameModes/Core/BP_Core_Character.BP_Core_Character_C|GetSpringArm _as_bp_core_character)))) (+ _returnvalue (* _returnvalue_2 (Variables|Default|GetShootingRange))) "TraceTypeQuery1" false (Utilities|Array|MakeArray (Variables|Default|GetAs%20BP%20Core%20Character)) "None"))
  (if _returnvalue_3
    (CallFunction|MCSpawnImpact (.Location (Collision|BreakHitResult _outhit)) (.Normal (Collision|BreakHitResult _outhit)))
    (Game|Damage|ApplyDamage (.HitActor (Collision|BreakHitResult _outhit)) (Variables|Default|GetDamage) (Game|GetInstigatorController (Variables|Default|GetAs%20BP%20Core%20Character)) self)))