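; BP_LootBox_Spawner is a level actor that scatters a random number of BP_LootCrate actors inside its box area.
; On BeginPlay, only the authority rolls the count, loops SpawnLoot through a DoN node, then destroys the spawner.
; SpawnLoot traces down on Visibility from random box points and places crates at hits, aligned to the surface normal.
; Missed traces still count toward the total.
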(event EventBeginPlay
  (Networking|SwitchHasAuthority
    (:Authority
      (Variables|Default|SetAmountOfLoot (Math|Random|RandomIntegerinRange 15 25))
      (bind _counter (Utilities|FlowControl|DoN (Variables|Default|GetAmountOfLoot) :!label _label)
        (:Exit
          (CallFunction|SpawnLoot)
          (if (== _counter (Variables|Default|GetAmountOfLoot))
            (Actor|DestroyActor)
            (else
              (goto _label))))))))

(fn ConstructionScript)

(fn SpawnLoot
  (bind _box (Variables|Default|GetBox))
  (bind _box_2 (Variables|Default|GetBox))
  (bind _returnvalue (Components|Box|GetUnscaledBoxExtent _box_2))
  (bind _returnvalue_2 (Transformation|GetWorldLocation _box))
  (bind _returnvalue_3 (Math|Random|RandomPointinBoundingBox _returnvalue_2 _returnvalue))
  (bind (_x _y) (Math|Vector|BreakVector _returnvalue_3))
  (bind (_outhit _returnvalue_4) (Collision|LineTraceByChannel _returnvalue_3 (Math|Vector|MakeVector _x _y -2e+03) "TraceTypeQuery1" false 0 "None"))
  (if _returnvalue_4
    (Game|SpawnActorfromClass "/Game/Blueprints/Actors/BP_LootCrate.BP_LootCrate_C" (Math|Transform|MakeTransform (.Location (Collision|BreakHitResult _outhit)) (Math|Rotator|MakeRotator (.Roll (Math|Rotator|BreakRotator (Math|Conversions|RotationFromXVector (.Normal (Collision|BreakHitResult _outhit))))) (- (.Pitch (Math|Rotator|BreakRotator (Math|Conversions|RotationFromXVector (.Normal (Collision|BreakHitResult _outhit))))) 9e+01) (.Yaw (Math|Rotator|BreakRotator (Math|Conversions|RotationFromXVector (.Normal (Collision|BreakHitResult _outhit))))))) "Undefined" 0 0)))