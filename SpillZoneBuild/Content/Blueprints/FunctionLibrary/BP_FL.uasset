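; BP_FL is a function library of shared helpers for session exit, kill feed messages and player appearance saves.
; LeaveSession forwards to BP_GI, and AddKillFeed pushes text to every WB_KillFeedPanel widget after checking that player controller 0 is local.
; SaveAppearance writes a fresh BSG_Appearance holding the hat ID to a save slot.
; LoadAppearance reads it back, returning a success flag and the ID.
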(fn LeaveSession
  (bind _asbp_gi (Utilities|Casting|CastToBP_GI (Game|GetGameInstance)))
  (Default|LeaveSession _asbp_gi))

(fn AddKillFeed
  (params (Feedback_Text :type Text))
  (if (Pawn|IsLocalController (Game|GetPlayerController 0))
    (bind _foundwidgets (Widget|GetAllWidgetsOfClass 0 "/Game/Widgets/GameWidgets/Killfeed/WB_KillFeedPanel.WB_KillFeedPanel_C" false))
    (if (Utilities|Array|IsNotEmpty _foundwidgets)
      (for _array_element _foundwidgets
        (Default|AddKillfeed _array_element Feedback_Text)))))

(fn LoadAppearance
  (bind _returnvalue (SaveGame|DoesSaveGameExist "Appearance"))
  (if _returnvalue
    (bind _returnvalue_2 (SaveGame|LoadGamefromSlot "Appearance"))
    (bind _asbsg_appearance (Utilities|Casting|CastToBSG_Appearance _returnvalue_2)
      (:then
        (return true (Variables|/Game/Blueprints/SaveGame/BSG_Appearance.BSG_Appearance_C|GetHat_ID _asbsg_appearance)))
      (:CastFailed
        _)))
  (return false ""))

(fn SaveAppearance
  (params (Hat_ID :type String))
  (bind _returnvalue (SaveGame|CreateSaveGameObject "/Game/Blueprints/SaveGame/BSG_Appearance.BSG_Appearance_C"))
  (bind _output_get (LocalVariables|SetSaveGameObject _returnvalue))
  (Variables|/Game/Blueprints/SaveGame/BSG_Appearance.BSG_Appearance_C|SetHat_ID _output_get Hat_ID)
  (SaveGame|SaveGametoSlot (LocalVariables|GetSaveGameObject) "Appearance")
  (return))