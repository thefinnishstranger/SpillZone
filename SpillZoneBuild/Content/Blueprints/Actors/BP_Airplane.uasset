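; BP_Airplane is an actor that carries the gameplay characters at the start of its run and removes itself after traveling far enough.
; On BeginPlay, the server records the start location and teleports every BP_Gameplay_Character to a random point inside the plane's Box component.
; Each Tick, the server destroys the plane once it is at least 70,000 units from that start location.
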(event EventBeginPlay
  (Networking|SwitchHasAuthority
    (:Authority
      (Variables|Default|SetStartLocation (Transformation|GetActorLocation))
      (CallFunction|SpawnPlayersinPlane))))

(event EventTick
  (params (DeltaSeconds :type Float%20%28single-precision%29))
  (Networking|SwitchHasAuthority
    (:Authority
      (if (>= (Math|Vector|Distance(Vector) (Variables|Default|GetStartLocation) (Transformation|GetActorLocation)) 7e+04)
        (Actor|DestroyActor)))))

(fn ConstructionScript)

(fn SpawnPlayersinPlane
  (bind _outactors (Actor|GetAllActorsOfClass "/Game/Blueprints/GameModes/Gameplay/BP_Gameplay_Character.BP_Gameplay_Character_C"))
  (for _array_element _outactors
    (Transformation|SetActorLocation _array_element (Math|Random|RandomPointinBoundingBox (Transformation|GetWorldLocation (Variables|Default|GetBox)) (Variables|/Script/Engine.BoxComponent|GetBoxExtent (Variables|Default|GetBox))) false true)))