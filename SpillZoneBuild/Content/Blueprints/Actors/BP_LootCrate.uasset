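; Interactable loot crate that opens once and spawns one to three random pickup items inside its spawning volume.
; The Opened RepNotify drives a timeline that rotates the lid, while the multicast cosmetic opening event is empty.
; Each spawn draws random DT_PickupItems rows until one passes its SpawnPercentage roll, then spawns BP_PickupItem with that ID.
; Focus briefly shows a "Lootcrate" interaction widget, using a retriggerable delay to hide it.
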(event Custom|OpenCrate
  ;[1 1 1] Event responsible for opening lid
  (bind _lidrotation (Timeline|CrateOpening_Timeline PlayFromStart)
    (:Update
      (Transformation|SetRelativeRotation (Variables|Default|GetLid) (Math|Rotator|MakeRotator _lidrotation 0.0 0.0) false false))))

(event Custom|MC_CosmeticOpening
  ;[1 1 1] Handle Cosmetic events
)

(event Custom|SpawnItems
  (bind _output_get (Variables|Default|SetLootSpawnAmount (Math|Random|RandomIntegerinRange 1 3)))
  (bind _counter (Utilities|FlowControl|DoN _output_get :!label _label)
    (:Exit
      (CallFunction|SpawnActualItem)
      (if (not (== _counter (Variables|Default|GetLootSpawnAmount)))
        (goto _label)))))

(event Custom|SpawnActualItem
  (bind _outrownames (DataTable|GetDataTableRowNames "/Game/Blueprints/Data/PickupItems/DT_PickupItems.DT_PickupItems" :!label _label))
  (bind _returnvalue (Utilities|GetDataTableRow "/Game/Blueprints/Data/PickupItems/DT_PickupItems.DT_PickupItems" (.OutItem (Utilities|Array|Random _outrownames)))
    (:then
      (if (<= (Math|Random|RandomFloatinRange 0.0 1e+02) (.SpawnPercentage (Utilities|Struct|BreakS_PickupItem _returnvalue)))
        (Game|SpawnActorfromClass "/Game/Blueprints/Actors/BP_PickupItem.BP_PickupItem_C" (Math|Transform|MakeTransform (Math|Random|RandomPointinBoundingBox (Transformation|GetWorldLocation (Variables|Default|GetSpawningVolume)) (Components|Box|GetUnscaledBoxExtent (Variables|Default|GetSpawningVolume)))) "AdjustIfPossibleButAlwaysSpawn" 0 (.ID (Utilities|Struct|BreakS_PickupItem _returnvalue)) 0)
        (else
          (goto _label))))))

(event EventInteract
  (params (InteractingActor :type Actor%20Object%20Reference))
  (if (not (Variables|Default|GetOpened?))
    (Variables|Default|SetOpened? true)
    (CallFunction|MCCosmeticOpening)
    (CallFunction|SpawnItems)))

(event EventSetFocused
  (Rendering|SetVisibility (Variables|Default|GetWidget) true false)
  (Utilities|FlowControl|RetriggerableDelay 0.1)
  (Rendering|SetVisibility (Variables|Default|GetWidget) false false))

(event EventBeginPlay
  (CallFunction|SetupInteractionWidget))

(fn ConstructionScript)

(fn SetupInteractionWidget
  (bind _aswb_interaction_feedback (Utilities|Casting|CastToWB_InteractionFeedback (UserInterface|GetWidget (Variables|Default|GetWidget))))
  (Default|UpdateWidget _aswb_interaction_feedback "Lootcrate"))

(fn OnRepOpened?
  (CallFunction|OpenCrate))