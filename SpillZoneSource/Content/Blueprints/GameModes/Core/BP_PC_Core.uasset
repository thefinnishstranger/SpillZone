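; BP_PC_Core is a player controller that toggles the in-game menu from an input action and starts play in game-only input mode.
; ToggleGameMenu creates the WB_GameMenu widget on first use and adds it to the viewport, then reuses it by switching visibility between Visible and Collapsed.
; FocusWidget and FocusGame pair each menu state with the matching mouse cursor and input mode.
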(event EventBeginPlay
  (Input|SetInputModeGameOnly self))

(event Input|ActionEvents|InputActionToggleGameMenu
  (params (Key :type Key%20Structure :default "None"))
  (:Pressed
    (Widgets|ToggleGameMenu)))

(fn ConstructionScript)

(fn FocusWidget
  (Variables|Default|SetbShowMouseCursor true)
  (Input|SetInputModeGameandUI self (Variables|Default|GetWB_GameMenu) "DoNotLock" true))

(fn FocusGame
  (Variables|Default|SetbShowMouseCursor false)
  (Input|SetInputModeGameOnly self))

(fn ToggleGameMenu
  ;[1 1 1] Toggle Game menu
  (Variables|Default|GetWB_GameMenu
    (:then
      (if (Widget|IsVisible (Variables|Default|GetWB_GameMenu))
        (Widget|SetVisibility (Variables|Default|GetWB_GameMenu) "Collapsed")
        (Widgets|FocusGame)
        (else
          (Widget|SetVisibility (Variables|Default|GetWB_GameMenu) "Visible")
          (Widgets|FocusWidget))))
    (:else
      (bind _returnvalue (UserInterface|CreateWidget "/Game/Widgets/GameWidgets/WB_GameMenu.WB_GameMenu_C" self))
      (bind _output_get (Variables|Default|SetWB_GameMenu _returnvalue))
      (UserInterface|Viewport|AddtoViewport _output_get 0)
      (Widgets|FocusWidget))))